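; Shield pickup in the GASHandsOn project, built on a parent pickup class that provides the pickup and respawn events.
; It overrides CanBePickedUp to require both the parent check and a character whose shield is below its maximum.
; The picked-up and respawned events call the parent, then switch the particle system off and back on to match availability.
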(event `self.OnPickedUp`
  (`parent.OnPickedUp`)
  (`ActorComponent.Deactivate` (`self.ParticleSystem`)))

(event `self.OnRespawned`
  (`parent.OnRespawned`)
  (`ActorComponent.Activate` (`self.ParticleSystem`) true))

(fn `CanBePickedUp`
  (params (TestCharacter :type "GHOCharacterBase Object Reference"))
  (returns (ReturnValue :type Boolean))
  (bind _returnvalue (`parent.CanBePickedUp` TestCharacter))
  (if _returnvalue
    (return (< (`GHOCharacterBase.GetShield` TestCharacter) (`GHOCharacterBase.GetMaxShield` TestCharacter)))
    (else
      (return false))))

(fn `UserConstructionScript`)