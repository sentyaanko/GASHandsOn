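; Base meteor gameplay ability for heroes that drops a damaging projectile on a player-targeted location.
; Activation shows confirm/cancel UI, raises the camera boom and waits for user-confirmed target data.
; On confirmation it commits, and only the authority spawns the meteor above the hit point, passing it a SetByCaller damage spec plus additional effect specs.
; Cancelling or a failed commit cancels the ability; ending restores camera and UI.
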(event `self.K2_ActivateAbility`
  (bind _asghohero_character_base (cast `GHOHeroCharacterBase` (`self.GetAvatarActorFromActorInfo`)))
  (set `self.AvatarActor` _asghohero_character_base)
  (bind _isvalid (`self.ShowConfirmUI` true))
  (if _isvalid
    (`self.SetCameraBoomRelativeLocation` (0.0 0.0 100.0))
    (bind (_asynctaskproxy _data) (`AbilityTask_WaitTargetData.WaitTargetData` "None" "UserConfirmed" (`self.TargetActorClass`) 0.0 0.0 (`self.Max Range`) (struct :`Name` "TargetActorGroundLocation") true (`self.MakeTargetLocationInfoFromOwnerActor`) (struct) null)
      (:`ValidData`
        (bind _returnvalue (`self.K2_CommitAbility`))
        (if _returnvalue
          (if (`Actor.HasAuthority` (`self.AvatarActor`))
            (`self.SpawnMeteorProjectile` _data))
          (`self.K2_EndAbility`)
          (else
            (`self.K2_CancelAbility` :!label _label))))
      (:`Cancelled`
        (goto _label)))))

(event `self.K2_OnEndAbility`
  (params (bWasCancelled :type Boolean))
  (`self.SetCameraBoomRelativeLocation` (0.0 0.0 0.0))
  (`self.ShowConfirmUI` false))

(fn `MakeAdditionalEffectSpecs`
  (returns (NewParam :type "Array of GameplayEffectSpecHandle Structure"))
  (locals (EffectSpecs :type "Array of GameplayEffectSpecHandle Structure") (AbilityLevel :type "Float (double-precision)" :default 0.0))
  (set `local.AbilityLevel` (`KismetMathLibrary.Conv_IntToDouble` (`self.GetAbilityLevel`)))
  (for _array_element (`self.AdditionalGameplayEffectClasses`)
    (if (`KismetSystemLibrary.IsValidClass` _array_element)
      (`KismetArrayLibrary.Array_Add` (`local.EffectSpecs`) (`self.MakeOutgoingGameplayEffectSpec` _array_element (`local.AbilityLevel`)))))
  (return (`local.EffectSpecs`)))

(fn `MakeDamageEffectSpec`
  (returns (ReturnValue :type "GameplayEffectSpecHandle Structure"))
  (bind _returnvalue (`AbilitySystemBlueprintLibrary.AssignTagSetByCallerMagnitude` (`self.MakeOutgoingGameplayEffectSpec` (`self.DamageGameplayEffectClass`) (`KismetMathLibrary.Conv_IntToDouble` (`self.GetAbilityLevel`))) (struct :`TagName` "Data.Damage") (`self.DamageMagnitude`)))
  (return _returnvalue))

(fn `SetCameraBoomRelativeLocation`
  (params (Offset :type "Vector Structure"))
  (bind _avataractor (`self.AvatarActor`))
  (`SceneComponent.K2_SetRelativeLocation` (`GHOHeroCharacterBase.CameraBoom` _avataractor) (+ Offset (`GHOHeroCharacterBase.StartingCameraBoomRelativeLocation` _avataractor)) false false)
  (return))

(fn `ShowConfirmUI`
  (params (bShow :type Boolean))
  (returns (IsValid :type Boolean))
  (bind _asghoplayer_state (cast `GHOPlayerState` (`self.GetOwningActorFromActorInfo`))
    (:`then`
      (`GHOPlayerState.ShowAbilityConfirmCancelText` _asghoplayer_state bShow)
      (return true))
    (:`CastFailed`
      (return false))))

(fn `SpawnMeteorProjectile`
  (params (HitResult :type "GameplayAbilityTargetDataHandle Structure (by ref)"))
  (bind (_returnvalue_bblockinghit _returnvalue_binitialoverlap _returnvalue_time _returnvalue_distance _returnvalue_location) (`GameplayStatics.BreakHitResult` (`AbilitySystemBlueprintLibrary.GetHitResultFromTargetData` HitResult)))
  (bind _avataractor (`self.AvatarActor`))
  (bind _returnvalue (`self.MakeDamageEffectSpec`))
  (bind _newparam (`self.MakeAdditionalEffectSpecs`))
  (`|SpawnActorFromClass` (`self.MeteorProjectileClass`) (`KismetMathLibrary.MakeTransform` (+ _returnvalue_location (0.0 0.0 1000.0))) "AlwaysSpawn" "OverrideRootScale" _avataractor 0.0 _returnvalue _newparam _avataractor)
  (return))