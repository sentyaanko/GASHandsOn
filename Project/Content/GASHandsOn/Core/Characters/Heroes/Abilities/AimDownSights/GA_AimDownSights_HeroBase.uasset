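; Base aim-down-sights gameplay ability for heroes, zooming the camera and toggling the aiming state on the character's movement component.
; Initialization caches the hero avatar, then start and stop hooks switch the camera boom between zoomed and starting arm lengths.
; Movement hooks start and stop aim-down-sights, while pre/post removal hooks apply and remove a removal GameplayEffect.
; A stack-checked removal variant is left unconnected.
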(fn `Initialize BP`
  (returns (IsVlaid :type Boolean))
  (bind _asghohero_character_base (cast `GHOHeroCharacterBase` (`self.GetAvatarActorFromActorInfo`))
    (:`then`
      (set `self.OwningHero` _asghohero_character_base)
      (return true))
    (:`CastFailed`
      (return false))))

(fn `PostRemoveGameplayEffect`
  (`self.RemoveRemovalGameplayEffect`)
  (return))

(fn `PreRemoveGameplayEffect`
  (`self.ApplyRemovalGameplayEffect`)
  (return))

(fn `SetTargetArmLength`
  (params (TargetArmLength :type "Float (double-precision)"))
  (set `SpringArmComponent.TargetArmLength` TargetArmLength (`GHOHeroCharacterBase.CameraBoom` (`self.OwningHero`)))
  (return))

(fn `StartFunction`
  (params (CharacterMovementComponent :type "GHOCharacterMovementComponent Object Reference"))
  (`GHOCharacterMovementComponent.StartAimDownSights` CharacterMovementComponent)
  (return))

(fn `StartFunctionBP`
  (locals (Length :type "Float (double-precision)" :default 100.0))
  (`self.SetTargetArmLength` (`self.ZoomingCameraBoomTargetArmLength`))
  (return))

(fn `StopFunction`
  (params (CharacterMovementComponent :type "GHOCharacterMovementComponent Object Reference"))
  (`GHOCharacterMovementComponent.StopAimDownSights` CharacterMovementComponent)
  (return))

(fn `StopFunctionBP`
  (`self.SetTargetArmLength` (`GHOHeroCharacterBase.StartingCameraBoomTargetArmLength` (`self.OwningHero`)))
  (return))