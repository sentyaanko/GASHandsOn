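; GA_Sprint_HeroBase is the base hero sprint Gameplay Ability, starting and stopping sprint on the GHO character movement component with a locally added gameplay cue.
; While active, CheckCost loops on a short delay plus a server-wait net sync.
; Each tick commits the ability cost only when the hero is accelerating and not falling, and ends the ability if the commit fails.
; Overrides also apply and remove a removal gameplay effect.
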(event `self.CheckCost`
  (`AbilityTask_WaitDelay.WaitDelay` 0.05 :!label _label
    (:`OnFinish`
      (`AbilityTask_NetworkSyncPoint.WaitNetSync` "OnlyServerWait"
        (:`OnSync`
          (bind _asghocharacter_movement_component (`self.Get GHOCharacter Movement Component`))
          (`/Engine/EditorBlueprintResources/StandardMacros.IsValid` _asghocharacter_movement_component
            (:`Is Valid`
              (if (`self.IsNeedSprintCost` _asghocharacter_movement_component)
                (bind _returnvalue (`self.K2_CommitAbilityCost` false))
                (if _returnvalue
                  (if (`self.bActive`) :!label _label_2
                    (goto _label))
                  (else
                    (`self.CallEndAbility`)))
                (else
                  (goto _label_2))))))))))

(fn `CallEndAbility`
  (if (`self.bActive`)
    (set `self.bActive` false)
    (`parent.CallEndAbility`))
  (return))

(fn `Initialize BP`
  (returns (IsVlaid :type Boolean))
  (set `self.bActive` true)
  (return true))

(fn `IsNeedSprintCost`
  (params (CharacterMovementComponent :type "GHOCharacterMovementComponent Object Reference"))
  (returns (ReturnValue :type Boolean))
  (return (and (> (`KismetMathLibrary.VSize` (`CharacterMovementComponent.GetCurrentAcceleration` CharacterMovementComponent)) 0.0) (not (`NavMovementComponent.IsFalling` CharacterMovementComponent)))))

(fn `PostRemoveGameplayEffect`
  (`self.RemoveRemovalGameplayEffect`)
  (return))

(fn `PreRemoveGameplayEffect`
  (`self.ApplyRemovalGameplayEffect`)
  (return))

(fn `StartFunction`
  (params (CharacterMovementComponent :type "GHOCharacterMovementComponent Object Reference"))
  (`GHOCharacterMovementComponent.StartSprinting` CharacterMovementComponent)
  (bind _asghoability_system_component (cast `GHOAbilitySystemComponent` (`.AbilitySystemComponent` (break `GameplayAbilityActorInfo` (`self.GetActorInfo`))))
    (:`then`
      (`KismetSystemLibrary.PrintString` "Call AddGameplayCueLocal")
      (`GHOAbilitySystemComponent.AddGameplayCueLocal` :`self` _asghoability_system_component :`GameplayCueTag` (`self.GameplayCueTag`)))
    (:`CastFailed`
      _))
  (return))

(fn `StartFunctionBP`
  (return))

(fn `StopFunction`
  (params (CharacterMovementComponent :type "GHOCharacterMovementComponent Object Reference"))
  (`GHOCharacterMovementComponent.StopSprinting` CharacterMovementComponent)
  (bind _asghoability_system_component (cast `GHOAbilitySystemComponent` (`.AbilitySystemComponent` (break `GameplayAbilityActorInfo` (`self.GetActorInfo`))))
    (:`then`
      (`GHOAbilitySystemComponent.RemoveGameplayCueLocal` :`self` _asghoability_system_component :`GameplayCueTag` (`self.GameplayCueTag`)))
    (:`CastFailed`
      _))
  (return))