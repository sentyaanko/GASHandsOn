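; GA_NextWeapon is a gameplay ability that switches a hero character's weapon, with an IsPrevious variable passed as the direction.
; It can only activate when the avatar is a GHOHeroCharacterBase carrying more than one weapon.
; On activation it calls SwitchWeapon, applies GE_WeaponIsChangingDelayReplicationTag to block CurrentWeapon replication slightly beyond the equip montage, then ends immediately.
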(event `self.K2_ActivateAbility`
  (bind _asghohero_character_base (cast `GHOHeroCharacterBase` (`self.GetAvatarActorFromActorInfo`)))
  (`GHOHeroCharacterBase.SwitchWeapon` _asghohero_character_base (`self.bIsPrevious`))
  (`self.BP_ApplyGameplayEffectToOwner` "/Game/GASHandsOn/Core/Characters/Heroes/Abilities/SwitchWeapon/GE_WeaponIsChangingDelayReplicationTag.GE_WeaponIsChangingDelayReplicationTag_C") ; Equip montages are about 0.5s, this tag will last 1.5s. This gives us 1s of extra time that the CurrentWeapon is not allowed to replicate.\nEquip montage は約 0.5 秒、このタグは 1.5 秒持続します。これにより、 CurrentWeapon のレプリケーションが許可されない 1 秒の特別な時間が得られます。
  (`self.K2_EndAbility`))

(fn `K2_CanActivateAbility`
  (params (ActorInfo :type "GameplayAbilityActorInfo Structure"))
  (returns (RelevantTags :type "GameplayTagContainer Structure") (ReturnValue :type Boolean))
  (bind _asghohero_character_base (cast `GHOHeroCharacterBase` ActorInfo_AvatarActor)
    (:`then`
      (return (struct) (> (`GHOHeroCharacterBase.GetNumWeapons` _asghohero_character_base) 1)))
    (:`CastFailed`
      (return (struct) false))))