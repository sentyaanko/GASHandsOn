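; Gameplay ability that runs on a downed hero being revived, playing the revive animation and returning to the death montage if cancelled.
; It scales the montage play rate so the animation spans the hero's ReviveDuration, then ends when the montage completes.
; GE_Reviving is applied to the owner while the ability runs and removed by stored handle on end.
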(event `self.K2_ActivateAbility`
  (bind _revivemontage (`self.ReviveMontage`))
  (bind _asghohero_character_base (cast `GHOHeroCharacterBase` (`self.GetAvatarActorFromActorInfo`)))
  (bind _returnvalue (`AnimSequenceBase.GetPlayLength` _revivemontage))
  (`AbilityTask_PlayMontageAndWait.CreatePlayMontageAndWaitProxy` "None" _revivemontage (/ _returnvalue (`GHOHeroCharacterBase.ReviveDuration` _asghohero_character_base)) "None" false
    (:`then`
      (bind _returnvalue_2 (`self.BP_ApplyGameplayEffectToOwner` "/Game/GASHandsOn/Core/Characters/Shared/Abilities/Interact/Revive/GE_Reviving.GE_Reviving_C"))
      (set `self.GE_RevivingHandle` _returnvalue_2))
    (:`OnCompleted`
      (`self.K2_EndAbility`))))

(event `self.K2_OnEndAbility`
  (params (bWasCancelled :type Boolean))
  (`self.BP_RemoveGameplayEffectFromOwnerWithHandle` (`self.GE_RevivingHandle`))
  (if bWasCancelled
    (`AbilityTask_PlayMontageAndWait.CreatePlayMontageAndWaitProxy` "None" (`self.DeathMontage`) 1.0 "None" false)))