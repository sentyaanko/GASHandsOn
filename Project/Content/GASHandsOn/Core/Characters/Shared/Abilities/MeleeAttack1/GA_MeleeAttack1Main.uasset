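; Gameplay ability for a montage-driven melee combo, triggered by an input gameplay event and adding loose tags to block other abilities until it ends.
; Repeat input events inside a permission window are buffered until a section name is set, then jump the montage.
; Hit-box calls apply effect containers with SetByCaller damage from GetDamageMagnitude, which returns zero here.
; An alternative PlayMontageAndWaitForEvent path for externally sent hit events is left unconnected.
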(event `self.K2_ActivateAbilityFromEvent`
  (params (EventData :type "GameplayEventData Structure (by ref)"))
  (bind _inputeventtag (`self.InputEventTag`))
  (bind (_owneractor _avataractor _playercontroller _abilitysystemcomponent) (break `GameplayAbilityActorInfo` (`self.GetActorInfo`)))
  (if (== (`.EventTag` (break `GameplayEventData` EventData)) _inputeventtag)
    (`/Engine/EditorBlueprintResources/StandardMacros.IsValid` (`self.Montage`)
      (:`Is Valid`
        (bind _returnvalue (`self.K2_CommitAbility`))
        (if _returnvalue
          (bind _asghoability_system_component (cast `GHOAbilitySystemComponent` _abilitysystemcomponent)
            (:`then`
              (`/Engine/EditorBlueprintResources/StandardMacros.IsValid` _playercontroller
                (:`Is Valid`
                  (if (`Controller.IsLocalController` _playercontroller)
                    (`GHOAbilitySystemComponent.K2_AddLooseGameplayTags` _asghoability_system_component (`self.BlockOtherAbilityLooseTags`) 1 :!label _label)))
                (:`Is Not Valid`
                  (goto _label)))
              (`self.OnInputMeleeAttack`)
              (bind _asynctaskproxy (`AbilityTask_WaitGameplayEvent.WaitGameplayEvent` _inputeventtag null)
                (:`then`
                  (set `self.WaitGameplayEventAsyncTask` _asynctaskproxy))
                (:`EventReceived`
                  (`self.OnInputMeleeAttack`))))
            (:`CastFailed`
              (`self.K2_CancelAbility` :!label _label_2)))
          (else
            (goto _label_2))))
      (:`Is Not Valid`
        (goto _label_2)))
    (else
      (goto _label_2))))

(event `self.K2_OnEndAbility`
  (params (bWasCancelled :type Boolean))
  (bind (_owneractor _avataractor _playercontroller _abilitysystemcomponent) (break `GameplayAbilityActorInfo` (`self.GetActorInfo`)))
  (bind _asghoability_system_component (cast `GHOAbilitySystemComponent` _abilitysystemcomponent)
    (:`then`
      (`/Engine/EditorBlueprintResources/StandardMacros.IsValid` _playercontroller
        (:`Is Valid`
          (if (`Controller.IsLocalController` _playercontroller)
            (`GHOAbilitySystemComponent.K2_RemoveLooseGameplayTags` _asghoability_system_component (`self.BlockOtherAbilityLooseTags`) 1 :!label _label_3)))
        (:`Is Not Valid`
          (goto _label_3))))
    (:`CastFailed`
      _))
  (bind _playmontageandwaitforeventasynctask (`self.PlayMontageAndWaitForEventAsyncTask`)
    (:`then`
      (`GameplayTask.EndTask` _playmontageandwaitforeventasynctask))
    (:`else`
      _))
  (bind _playmontageandwaitasynctask (`self.PlayMontageAndWaitAsyncTask`)
    (:`then`
      (`GameplayTask.EndTask` _playmontageandwaitasynctask))
    (:`else`
      _))
  (bind _waitgameplayeventasynctask (`self.WaitGameplayEventAsyncTask`)
    (:`then`
      (`GameplayTask.EndTask` _waitgameplayeventasynctask))
    (:`else`
      _))
  (set `self.bPlayingMontage` false)
  (set `self.bInputPermission` false)
  (set `self.bInput` false)
  (set `self.JumpSectionName` "None"))

(event `OnInputMeleeAttack`
  (if (`self.bPlayingMontage`)
    (if (`self.bInputPermission`)
      (set `self.bInput` true)
      (`self.CheckAndJumpMontage`))
    (else
      (set `self.bInputPermission` false)
      (set `self.bInput` false)
      (set `self.JumpSectionName` "None")
      ;[1 1 1] GA の外からイベントを呼ばず、 ApplyHitBoxEventByAttackType を呼び出す場合はこちらを使う。
      (bind _asynctaskproxy (`AbilityTask_PlayMontageAndWait.CreatePlayMontageAndWaitProxy` "None" (`self.Montage`))
        (:`then`
          (set `self.PlayMontageAndWaitAsyncTask` _asynctaskproxy)
          (set `self.bPlayingMontage` true))
        (:`OnCompleted`
          (`self.K2_EndAbility` :!label _label_4))
        (:`OnInterrupted`
          (goto _label_4))
        (:`OnCancelled`
          (goto _label_4))))))

(event `CheckAndJumpMontage`
  (bind _jumpsectionname (`self.JumpSectionName`))
  (if (and (`self.bInput`) (!= _jumpsectionname "None"))
    (bind _asghoability_system_component (cast `GHOAbilitySystemComponent` (`self.GetAbilitySystemComponentFromActorInfo`))
      (:`then`
        (`GHOAbilitySystemComponent.K2_CurrentMontageJumpToSection` _asghoability_system_component _jumpsectionname))
      (:`CastFailed`
        _))
    (set `self.bInput` false)
    (set `self.JumpSectionName` "None")))

(event `SetInputPermission`
  (params (bPermission :type Boolean))
  (set `self.bInputPermission` bPermission))

(event `SetJumpSectionName`
  (params (SectionName :type Name))
  (bind _output_get (set `self.JumpSectionName` SectionName))
  (if (!= _output_get "None")
    (`self.CheckAndJumpMontage`)))

(event `ApplyHitBoxEventByAttackType`
  (params (MeleeAttackType :type Byte))
  (bind _keys (`BlueprintMapLibrary.Map_Keys` (`self.EffectContainerMap`)))
  (`self.ApplyHitBoxEvent` (`|GetArrayItem` _keys) (make `GameplayEventData` (struct) null null null null (struct) (struct) (struct) 0.0 (`GHOBlueprintFunctionLibrary.AbilityTargetDataFromInt32` (`KismetMathLibrary.Conv_ByteToInt` MeleeAttackType)))))

(event `ApplyHitBoxEvent`
  (params (ContainerTag :type "GameplayTag Structure") (EventData :type "GameplayEventData Structure"))
  (bind _returnvalue (`self.MakeEffectContainerSpec` ContainerTag EventData))
  (`AbilitySystemBlueprintLibrary.AssignTagSetByCallerMagnitude` (`|GetArrayItem` (`.TargetGameplayEffectSpecs` (break `GHOGameplayEffectContainerSpec` _returnvalue))) (struct :`TagName` "Data.Damage") (`self.GetDamageMagnitude` EventData))
  (`self.ApplyEffectContainerSpec` _returnvalue))

(fn `GetDamageMagnitude`
  (params (GameplayEventData :type "GameplayEventData Structure (by ref)"))
  (returns (Value :type "Float (double-precision)"))
  (return 0.0))