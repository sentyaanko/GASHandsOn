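; Gameplay ability that makes a character dash along its forward direction.
; On activation it commits the ability, cancelling if that fails, then starts the dash montage and immediately applies a constant root motion force.
; Montage, strength and duration come from variables, and the velocity captured when the force starts is set again on finish.
; The ability ends when the force finishes, independent of montage completion.
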(event `self.K2_ActivateAbility`
  (bind _returnvalue (`self.GetAvatarActorFromActorInfo`))
  (bind _returnvalue_2 (`self.K2_CommitAbility`))
  (if _returnvalue_2
    (`GHOAbilityTask_PlayMontageAndWaitForEvent.PlayMontageAndWaitForEvent` "None" (`self.DashMontage`)
      (:`then`
        (`AbilityTask_ApplyRootMotionConstantForce.ApplyRootMotionConstantForce` "None" (`Actor.GetActorForwardVector` _returnvalue) (`self.DashForceStrength`) (`self.DashForceDuration`) false null "SetVelocity" (`Actor.GetVelocity` _returnvalue)
          (:`OnFinish`
            (`self.K2_EndAbility`)))))
    (else
      (`self.K2_CancelAbility`))))