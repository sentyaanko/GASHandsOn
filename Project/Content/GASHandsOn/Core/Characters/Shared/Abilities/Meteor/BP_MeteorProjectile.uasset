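; BP_MeteorProjectile is the projectile actor for the Meteor ability, dealing area effects through the Gameplay Ability System when it hits the ground.
; Its collision sphere treats overlaps with WorldStatic or WorldDynamic components as ground impact, then destroys the actor.
; On authority only, impact first applies the damage and additional effect spec handles to living characters inside the sphere, excluding the instigator.
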(event `self.ReceiveBeginPlay`)

(event `self.SphereCollision.OnComponentBeginOverlap`
  (params (OverlappedComponent :type "PrimitiveComponent Object Reference") (OtherActor :type "Actor Object Reference") (OtherComp :type "PrimitiveComponent Object Reference") (OtherBodyIndex :type Integer) (bFromSweep :type Boolean) (SweepResult :type "HitResult Structure (by ref)"))
  (if (`self.IsHitGround` OtherComp)
    (`/Engine/EditorBlueprintResources/ActorMacros.Switch Has Authority`
      (:`Authority`
        (`self.ApplyGameplayEffectToOverlapCharacters` (`self.GetInstigator`)))
      (:`Remote`
        _))
    (`self.K2_DestroyActor`)))

(fn `ApplyGameplayEffectToOverlapCharacters`
  (params (Instigator :type "Pawn Object Reference"))
  (for _array_element (`PrimitiveComponent.GetOverlappingActors` (`self.SphereCollision`) "/Script/GASHandsOn.GHOCharacterBase")
    (bind _asghocharacter_base (cast `GHOCharacterBase` _array_element))
    (bind _returnvalue (`AbilitySystemBlueprintLibrary.GetAbilitySystemComponent` _asghocharacter_base))
    (if (and (`KismetSystemLibrary.IsValid` _returnvalue) (`GHOCharacterBase.IsAlive` _asghocharacter_base) (!= _asghocharacter_base Instigator))
      (`AbilitySystemComponent.BP_ApplyGameplayEffectSpecToSelf` _returnvalue (`self.DamageEffectSpecHandle`))
      (for _array_element_2 (`self.AdditionalEffectSpecHandles`)
        (`AbilitySystemComponent.BP_ApplyGameplayEffectSpecToSelf` _returnvalue _array_element_2))))
  (return))

(fn `IsHitGround`
  (params (OtherComp :type "PrimitiveComponent Object Reference"))
  (returns (ReturnValue :type Boolean))
  (bind _returnvalue (`PrimitiveComponent.GetCollisionObjectType` OtherComp))
  (return (or (`|EnumEquality` _returnvalue "ECC_WorldStatic") (`|EnumEquality` _returnvalue "ECC_WorldDynamic"))))

(fn `UserConstructionScript`)