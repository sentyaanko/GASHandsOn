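; Base Gameplay Ability for held character movement actions such as Sprint, with empty hooks for children to start and stop behavior on GHOCharacterMovementComponent.
; Activation applies a tag-granting GameplayEffect, calls the start hooks and CheckCost, then ends on input release or, after a server-wait net sync, when CancelAbilityTag is added.
; Ending removes the effect and runs stop hooks.
; Optional removal-effect helpers let children predict tag removal, working around unpredictable GE removal.
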(event `self.K2_ActivateAbility`
  (bind _cancelabilitytag (`self.CancelAbilityTag`))
  (bind _isvlaid (`self.Initialize BP`))
  (if _isvlaid
    ;[1 1 1] Predictively apply GameplayTag.
    ; GameplayTag を Predictively （予測的）に適用する。
    ;
    ; GameplayEffectClass で指定されているクラスにて、このアビリティが適用されていることを示す GameplayTag を Add する。
    ; 例：Sprint の場合は "State.Sprinting" を付与する GameplayEffect を指定する。
    (bind _returnvalue (`self.BP_ApplyGameplayEffectToOwner` (`self.GameplayEffectClass`) (`self.GetAbilityLevel`)))
    (set `self.GameplayEffectHandle` _returnvalue)
    (`self.StartFunctionBP`)
    (bind _asghocharacter_movement_component (`self.Get GHOCharacter Movement Component`))
    (`/Engine/EditorBlueprintResources/StandardMacros.IsValid` _asghocharacter_movement_component
      (:`Is Valid`
        (`self.StartFunction` _asghocharacter_movement_component)
        (`AbilityTask_WaitInputRelease.WaitInputRelease` true
          (:`then`
            ;[1 1 1] Using the CancelAbilitiesWithTag AbilityTags doesn't create a new scoped prediction window which we need to predict our sprint removal in EndAbility.
            ; So we do it with a task instead.
            ;
            ; (GameplayAbility のプロパティの1つである)CancelAbilitiesWithTag AbilityTags を使用しても、 EndAbility の際にスプリントの削除を予測するために必要な、新しいスコープ付き予測ウィンドウが作成されません。
            ; そこで、代わりにタスクを使って行います。
            ;
            ; 詳しくは GASDocumentation の「4.10 Prediction （予測）」の見出し以下を参照。
            (if (`BlueprintGameplayTagLibrary.IsGameplayTagValid` _cancelabilitytag)
              (bind _asynctaskproxy (`AbilityTask_WaitGameplayTagAdded.WaitGameplayTagAdd` _cancelabilitytag null)
                (:`then`
                  (set `self.WaitGameplayTagAsyncTask` _asynctaskproxy)
                  (`self.CheckCost` :!label _label))
                (:`Added`
                  (`AbilityTask_NetworkSyncPoint.WaitNetSync` "OnlyServerWait"
                    (:`OnSync`
                      (`self.CallEndAbility` :!label _label_2)))))
              (else
                (goto _label))))
          (:`OnRelease`
            (goto _label_2)))))))

(event `self.K2_OnEndAbility`
  (params (bWasCancelled :type Boolean))
  ;[1 1 1] Predictively apply RemovalGameplayTag and remove GEs that give GameplayTag and RemovalGameplayTag.
  ; Both tags will still exist on the client (because we can't predictively remove GEs) until the Server's removal of the GEs replicates in.
  ; At that point both tags will be removed in the same frame.
  ; Whenever we check if we have GameplayTag, we're actually checking if the tag count for GameplayTag is > RemovalGameplayTag.
  ;
  ; 予測的に RemovalGameplayTag を適用し、 GameplayTag と RemovalGameplayTag を与える GE を削除する。
  ; 両方のタグは、（サーバーでの GE の削除がレプリケーションされるまでの間、）（GE を予測的に削除することが出来ないため、）クライアント上に依然として存在します。
  ; その時点（サーバーからレプリケーションされた時点）で、両方のタグは同じフレーム内で削除されます。
  ; GameplayTag があるかどうかのチェックをするときは、実際にはタグ数が GameplayTag > RemovalGameplayTag であるかどうかをチェックしています。
  ;
  ; ※GASShooter では、 Sprint の実装では上記のチェックしていません。
  ; ※これは、 Sprint では、事前に RemovalGameplayTag の付与を行わないためです。
  ; ※（キーを離すか、スタミナが尽きた時点で EndAbility を呼ぶかのどちらかしかありません。）
  ; ※（つまり、 Weapon と異なり、アビリティの終了が確定したが EndAbility の呼び出しは他の都合上少し遅れる、などがありません。）
  ; ※Weapon の セカンダリアビリティである AimDownSights ではチェックしています。
  ; ※ここでは Sprint / Weapon の両方の形式の関数を用意し、派生側で都合が良い方を呼び出して貰う形で実装します。
  ; ※（ Sprint のほうがコストが安いですが、 Weapon 形式でまとめても良い気がします）
  (`self.PreRemoveGameplayEffect`)
  (`self.BP_RemoveGameplayEffectFromOwnerWithHandle` (`self.GameplayEffectHandle`))
  (set `self.GameplayEffectHandle` (struct))
  (`self.PostRemoveGameplayEffect`)
  (`self.StopFunctionBP`)
  (bind _asghocharacter_movement_component (`self.Get GHOCharacter Movement Component`))
  (`/Engine/EditorBlueprintResources/StandardMacros.IsValid` _asghocharacter_movement_component
    (:`Is Valid`
      (`self.StopFunction` _asghocharacter_movement_component)
      (bind _waitgameplaytagasynctask (`self.WaitGameplayTagAsyncTask`)
        (:`then`
          (`GameplayTask.EndTask` _waitgameplaytagasynctask))
        (:`else`)))))

(event `CheckCost`)

(fn `ApplyRemovalGameplayEffect`
  (bind _returnvalue (`self.BP_ApplyGameplayEffectToOwner` (`self.GameplayEffectRemovalClass`) (`self.GetAbilityLevel`)))
  (set `self.GameplayEffectRemovalHandle` _returnvalue)
  (return))

(fn `ApplyRemovalGameplayEffectWithStackCheck`
  (bind _returnvalue (`AbilitySystemBlueprintLibrary.GetActiveGameplayEffectStackCount` (`self.GameplayEffectRemovalHandle`)))
  (if (not (> _returnvalue 0))
    (`self.ApplyRemovalGameplayEffect`))
  (return))

(fn `CallEndAbility`
  (`self.K2_EndAbility`)
  (return))

(fn `Get GHOCharacter Movement Component`
  (returns (`AsGHOCharacter Movement Component` :type "GHOCharacterMovementComponent Object Reference"))
  (bind (_returnvalue_owneractor _returnvalue_avataractor _returnvalue_playercontroller _returnvalue_abilitysystemcomponent _returnvalue_skeletalmeshcomponent _returnvalue_animinstance _returnvalue_movementcomponent) (break `GameplayAbilityActorInfo` (`self.GetActorInfo`)))
  (bind _asghocharacter_movement_component (cast `GHOCharacterMovementComponent` _returnvalue_movementcomponent)
    (:`then`
      (return _asghocharacter_movement_component))
    (:`CastFailed`
      (return null))))

(fn `Initialize BP`
  (returns (IsVlaid :type Boolean))
  (return true))

(fn `PostRemoveGameplayEffect`
  (return))

(fn `PreRemoveGameplayEffect`
  (return))

(fn `RemoveRemovalGameplayEffect`
  (`self.BP_RemoveGameplayEffectFromOwnerWithHandle` (`self.GameplayEffectRemovalHandle`))
  (set `self.GameplayEffectRemovalHandle` (struct))
  (return))

(fn `StartFunction`
  (params (CharacterMovementComponent :type "GHOCharacterMovementComponent Object Reference"))
  (return))

(fn `StartFunctionBP`
  (locals (Length :type "Float (double-precision)" :default 100.0))
  (return))

(fn `StopFunction`
  (params (CharacterMovementComponent :type "GHOCharacterMovementComponent Object Reference"))
  (return))

(fn `StopFunctionBP`
  (locals (Length :type "Float (double-precision)" :default 300.0))
  (return))