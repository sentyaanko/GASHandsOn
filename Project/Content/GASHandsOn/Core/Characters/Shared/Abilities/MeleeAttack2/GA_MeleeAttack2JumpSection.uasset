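; Gameplay ability, activated by event, that handles combo input for MeleeAttack2 by jumping the current montage to a section named in the event's target data.
; After committing, it watches two loose tags: the pushed-combo tag triggers the jump, while removal of the enable-jump tag closes the input window; either ends the ability.
; On end, it stops both wait tasks and clears all pushed-combo tag counts.
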(event `self.K2_ActivateAbilityFromEvent`
  (params (EventData :type "GameplayEventData Structure (by ref)"))
  (bind _returnvalue (`self.K2_CommitAbility`))
  (if _returnvalue
    (bind _asynctaskproxy (`AbilityTask_WaitGameplayTagRemoved.WaitGameplayTagRemove` (`self.LooseEnableComboJumpSectionTag`) null true) ; キー入力期間終了監視
      (:`then`
        (set `self.WaitEndJumpEnableSectionAsyncTask` _asynctaskproxy)
        (bind _asynctaskproxy_2 (`AbilityTask_WaitGameplayTagAdded.WaitGameplayTagAdd` (`self.LoosePushedComboTag`) null true) ; キーの入力待ち
          (:`then`
            (set `self.WaitPushedComboAsyncTask` _asynctaskproxy_2))
          (:`Added`
            (bind _asghoability_system_component (cast `GHOAbilitySystemComponent` (`self.GetAbilitySystemComponentFromActorInfo`))
              (:`then`
                (`GHOAbilitySystemComponent.K2_CurrentMontageJumpToSection` _asghoability_system_component (`GHOBlueprintFunctionLibrary.GetNameFromTargetData` (`.TargetData` (break `GameplayEventData` EventData)))))
              (:`CastFailed`
                _))
            (`self.K2_EndAbility`))))
      (:`Removed`
        (`self.K2_EndAbility`)))
    (else
      (`self.K2_CancelAbility`))))

(event `self.K2_OnEndAbility`
  (params (bWasCancelled :type Boolean))
  (bind _loosepushedcombotag (`self.LoosePushedComboTag`))
  (bind _waitendjumpenablesectionasynctask (`self.WaitEndJumpEnableSectionAsyncTask`)
    (:`then`
      (`GameplayTask.EndTask` _waitendjumpenablesectionasynctask))
    (:`else`
      _))
  (bind _waitpushedcomboasynctask (`self.WaitPushedComboAsyncTask`)
    (:`then`
      (`GameplayTask.EndTask` _waitpushedcomboasynctask))
    (:`else`
      _))
  (bind _asghoability_system_component (cast `GHOAbilitySystemComponent` (`self.GetAbilitySystemComponentFromActorInfo`)))
  (bind _returnvalue (`GHOAbilitySystemComponent.K2_GetTagCount` _asghoability_system_component _loosepushedcombotag))
  (if (!= _returnvalue 0)
    (`GHOAbilitySystemComponent.K2_RemoveLooseGameplayTag` _asghoability_system_component _loosepushedcombotag _returnvalue)))