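; GA_MeleeAttack2Damage is an event-activated gameplay ability that applies damage for the MeleeAttack2 set of character abilities.
; After committing, it builds an effect container spec from the event's tag and data, then sets Data.Damage by SetByCaller on the first effect spec.
; It applies the container and ends, or cancels if the commit fails.
; The magnitude comes from GetDamageMagnitude, which returns zero here.
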(event `self.K2_ActivateAbilityFromEvent`
  (params (EventData :type "GameplayEventData Structure (by ref)"))
  (bind _returnvalue (`self.K2_CommitAbility`))
  (if _returnvalue
    (bind _returnvalue_2 (`self.MakeEffectContainerSpec` (`.EventTag` (break `GameplayEventData` EventData)) EventData))
    (`AbilitySystemBlueprintLibrary.AssignTagSetByCallerMagnitude` (`|GetArrayItem` (`.TargetGameplayEffectSpecs` (break `GHOGameplayEffectContainerSpec` _returnvalue_2))) (struct :`TagName` "Data.Damage") (`self.GetDamageMagnitude` EventData))
    (`self.ApplyEffectContainerSpec` _returnvalue_2)
    (`self.K2_EndAbility`)
    (else
      (`self.K2_CancelAbility`))))

(fn `GetDamageMagnitude`
  (params (EventData :type "GameplayEventData Structure (by ref)"))
  (returns (DamageMagnitude :type "Float (double-precision)"))
  (return 0.0))