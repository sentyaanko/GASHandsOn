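; Gameplay ability for the first stage of a second melee attack, driven by gameplay events.
; After commit it adds a loose running-first tag, plus ability-blocking tags for local player controllers; non-local player controllers cancel, while pawns without one skip the blocking tags.
; It sends a play-montage event and ends on the end-montage event.
; Ending stops the wait task and removes the tags under the same controller checks.
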(event `self.K2_ActivateAbility`
  (bind (_owneractor _avataractor _playercontroller _abilitysystemcomponent) (break `GameplayAbilityActorInfo` (`self.GetActorInfo`)))
  (bind _returnvalue (`self.K2_CommitAbility`))
  (if _returnvalue
    (bind _asghoability_system_component (cast `GHOAbilitySystemComponent` _abilitysystemcomponent)
      (:`then`
        (`/Engine/EditorBlueprintResources/StandardMacros.IsValid` _playercontroller
          (:`Is Valid`
            (if (`Controller.IsLocalController` _playercontroller)
              (`GHOAbilitySystemComponent.K2_AddLooseGameplayTags` _asghoability_system_component (`self.BlockOtherAbilityLooseTags`) 1)
              (`GHOAbilitySystemComponent.K2_AddLooseGameplayTag` _asghoability_system_component (`self.LooseRunningFirstTag`) 1 :!label _label)
              (bind _asynctaskproxy (`AbilityTask_WaitGameplayEvent.WaitGameplayEvent` (`self.EndMontageEventTag`) null true)
                (:`then`
                  (set `self.WaitGameplayEventAsyncTask` _asynctaskproxy)
                  (`self.SendGameplayEvent` (`self.PlayMontageEventTag`)))
                (:`EventReceived`
                  (`self.K2_EndAbility`)))
              (else
                (`self.K2_CancelAbility` :!label _label_2))))
          (:`Is Not Valid`
            (goto _label))))
      (:`CastFailed`
        (goto _label_2)))
    (else
      (goto _label_2))))

(event `self.K2_OnEndAbility`
  (params (bWasCancelled :type Boolean))
  (bind (_owneractor _avataractor _playercontroller _abilitysystemcomponent) (break `GameplayAbilityActorInfo` (`self.GetActorInfo`)))
  (bind _waitgameplayeventasynctask (`self.WaitGameplayEventAsyncTask`)
    (:`then`
      (`GameplayTask.EndTask` _waitgameplayeventasynctask))
    (:`else`
      _))
  (bind _asghoability_system_component (cast `GHOAbilitySystemComponent` _abilitysystemcomponent))
  (`/Engine/EditorBlueprintResources/StandardMacros.IsValid` _playercontroller
    (:`Is Valid`
      (if (`Controller.IsLocalController` _playercontroller)
        (`GHOAbilitySystemComponent.K2_RemoveLooseGameplayTags` _asghoability_system_component (`self.BlockOtherAbilityLooseTags`) 1)
        (`GHOAbilitySystemComponent.K2_RemoveLooseGameplayTag` _asghoability_system_component (`self.LooseRunningFirstTag`) 1 :!label _label_3)))
    (:`Is Not Valid`
      (goto _label_3))))