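; Event-activated gameplay ability that plays a montage for the MeleeAttack2 melee attack.
; It commits, then runs a PlayMontageAndWait task and ends on completion, interruption or cancellation, or cancels if the commit fails.
; On end it stops the stored task and sends an end-montage gameplay event, only when a local player controller owns it.
; GetDamageMagnitude is a stub returning zero.
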(event `self.K2_ActivateAbilityFromEvent`
  (params (EventData :type "GameplayEventData Structure (by ref)"))
  (bind _returnvalue (`self.K2_CommitAbility`))
  (if _returnvalue
    (bind _asynctaskproxy (`AbilityTask_PlayMontageAndWait.CreatePlayMontageAndWaitProxy` "None" (`self.Montage`))
      (:`then`
        (set `self.PlayMontageAndWaitAsyncTask` _asynctaskproxy))
      (:`OnCompleted`
        (`self.K2_EndAbility` :!label _label))
      (:`OnInterrupted`
        (goto _label))
      (:`OnCancelled`
        (goto _label)))
    (else
      (`self.K2_CancelAbility`))))

(event `self.K2_OnEndAbility`
  (params (bWasCancelled :type Boolean))
  (bind (_returnvalue_owneractor _returnvalue_avataractor _returnvalue_playercontroller) (break `GameplayAbilityActorInfo` (`self.GetActorInfo`)))
  (bind _playmontageandwaitasynctask (`self.PlayMontageAndWaitAsyncTask`)
    (:`then`
      (`GameplayTask.EndTask` _playmontageandwaitasynctask))
    (:`else`
      _))
  (`/Engine/EditorBlueprintResources/StandardMacros.IsValid` _returnvalue_playercontroller
    (:`Is Valid`
      (if (`Controller.IsLocalController` _returnvalue_playercontroller)
        (`self.SendGameplayEvent` (`self.EndMontageEventTag`))))
    (:`Is Not Valid`)))

(fn `GetDamageMagnitude`
  (params (InputPin :type "GameplayEventData Structure"))
  (returns (OutputPin :type "Float (double-precision)"))
  (return 0.0))