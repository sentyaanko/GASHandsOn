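; GA_PassiveArmor is a passive Gameplay Ability that maintains stacking armor charges on its owner.
; A repeating WaitDelay applies one stack of the armor GameplayEffect per recharge interval, while each received damage event removes one stack by granted tag.
; A stack-change listener, bound once, stops recharging at StackMax and restarts it when the count leaves max.
; Ending the ability ends all three async tasks.
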(event `self.K2_ActivateAbility`
  (`self.StartRechargeWaitDelay`)
  (`/Engine/EditorBlueprintResources/StandardMacros.DoOnce` false
    (:`Completed`
      (bind _asynctaskproxy (`GHOAbilityTask_WaitReceiveDamage.WaitReceiveDamage` false)
        (:`then`
          (set `self.WaitReceiveDamageTask` _asynctaskproxy))
        (:`OnDamage`
          (`self.BP_RemoveGameplayEffectFromOwnerWithGrantedTags` (`self.RemoveGameplayEffectTag`) 1))))))

(event `StartRechargeWaitDelay`
  (bind _asynctaskproxy (`AbilityTask_WaitDelay.WaitDelay` (`self.RechargeDelay`))
    (:`then`
      (set `self.WaitDelayForRechargeTask` _asynctaskproxy))
    (:`OnFinish`
      (`self.OnFinishStartRechargeWaitDelay`))))

(event `OnFinishStartRechargeWaitDelay`
  (bind _returnvalue (`self.BP_ApplyGameplayEffectToOwner` (`self.GameplayEffectClass`) (`self.GetAbilityLevel`)))
  (`self.StartWaitForGameplayEffectStackChange` _returnvalue)
  (if (`self.bNeedCharge`)
    (`self.StartRechargeWaitDelay`)))

(event `StartWaitForGameplayEffectStackChange`
  (params (Handle :type "ActiveGameplayEffectHandle Structure"))
  (`/Engine/EditorBlueprintResources/StandardMacros.DoOnce` false
    (:`Completed`
      (bind (_asynctaskproxy _handle _newcount _oldcount) (`AbilityTask_WaitGameplayEffectStackChange.WaitForGameplayEffectStackChange` Handle)
        (:`then`
          (set `self.WaitStackChangeTask` _asynctaskproxy))
        (:`OnChange`
          (`self.OnChangeGameplayEffectStack` _newcount _oldcount))))))

(event `OnChangeGameplayEffectStack`
  (params (NewCount :type Integer) (OldCount :type Integer))
  (bind _stackmax (`self.StackMax`))
  (if (== NewCount _stackmax)
    (bind _waitdelayforrechargetask (`self.WaitDelayForRechargeTask`)
      (:`then`
        (`GameplayTask.EndTask` _waitdelayforrechargetask))
      (:`else`
        _))
    (set `self.bNeedCharge` false)
    (elif (== OldCount _stackmax)
      (set `self.bNeedCharge` true)
      (`self.StartRechargeWaitDelay`))))

(event `self.K2_OnEndAbility`
  (params (bWasCancelled :type Boolean))
  (bind _waitreceivedamagetask (`self.WaitReceiveDamageTask`)
    (:`then`
      (`GameplayTask.EndTask` _waitreceivedamagetask))
    (:`else`
      _))
  (bind _waitdelayforrechargetask (`self.WaitDelayForRechargeTask`)
    (:`then`
      (`GameplayTask.EndTask` _waitdelayforrechargetask))
    (:`else`
      _))
  (bind _waitstackchangetask (`self.WaitStackChangeTask`)
    (:`then`
      (`GameplayTask.EndTask` _waitstackchangetask))
    (:`else`)))