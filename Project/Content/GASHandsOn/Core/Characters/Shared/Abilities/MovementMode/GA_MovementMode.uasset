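; Gameplay ability that mirrors the character's current movement mode as a loose gameplay tag on its GHOAbilitySystemComponent.
; On activation it cancels for non-local player controllers or a missing CharacterMovementComponent; actors without a PlayerController proceed.
; It adds the initial tag, then re-arms WaitMovementModeChange after each change, swapping the stored tag for the new mode's.
; Ending the ability stops the wait task and removes the tag.
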(event `self.K2_ActivateAbility`
  (bind (_owneractor _avataractor _playercontroller _abilitysystemcomponent _skeletalmeshcomponent _animinstance _movementcomponent) (break `GameplayAbilityActorInfo` (`self.GetActorInfo`)))
  (`/Engine/EditorBlueprintResources/StandardMacros.IsValid` _playercontroller
    (:`Is Valid`
      (if (`Controller.IsLocalPlayerController` _playercontroller)
        (bind _ascharacter_movement_component (cast `CharacterMovementComponent` _movementcomponent :!label _label)
          (:`then`
            (`self.AddMovementModeGameplayTag` (`CharacterMovementComponent.MovementMode` _ascharacter_movement_component))
            (bind (_asynctaskproxy _newmovementmode) (`AbilityTask_WaitMovementModeChange.CreateWaitMovementModeChange` "MOVE_None" :!label _label_2)
              (:`then`
                (set `self.WaitMovementModeChangeAsyncTask` _asynctaskproxy))
              (:`OnChange`
                (`self.RemoveMovementModeGameplayTag`)
                (`self.AddMovementModeGameplayTag` _newmovementmode)
                (goto _label_2))))
          (:`CastFailed`
            (`self.K2_CancelAbility` :!label _label_3)))
        (else
          (goto _label_3))))
    (:`Is Not Valid`
      (goto _label))))

(event `self.K2_OnEndAbility`
  (params (bWasCancelled :type Boolean))
  (bind _waitmovementmodechangeasynctask (`self.WaitMovementModeChangeAsyncTask`)
    (:`then`
      (`GameplayTask.EndTask` _waitmovementmodechangeasynctask))
    (:`else`
      _))
  (`self.RemoveMovementModeGameplayTag`))

(fn `AddMovementModeGameplayTag`
  (params (MovementMode :type "EMovementMode Enum" :default "MOVE_None"))
  (bind _asghoability_system_component (cast `GHOAbilitySystemComponent` (`self.GetAbilitySystemComponentFromActorInfo`))
    (:`then`
      (bind _outputpin (`self.SelectMovementModeGameplayTag` MovementMode))
      (bind _output_get (set `self.AddedGameplayTag` _outputpin))
      (`GHOAbilitySystemComponent.K2_AddLooseGameplayTag` _asghoability_system_component _output_get 1))
    (:`CastFailed`
      (`KismetSystemLibrary.PrintString` "Add :ASC not found")))
  (return))

(fn `RemoveMovementModeGameplayTag`
  (bind _addedgameplaytag (`self.AddedGameplayTag`))
  (bind _asghoability_system_component (cast `GHOAbilitySystemComponent` (`self.GetAbilitySystemComponentFromActorInfo`))
    (:`then`
      (if (`BlueprintGameplayTagLibrary.IsGameplayTagValid` _addedgameplaytag)
        (`GHOAbilitySystemComponent.K2_RemoveLooseGameplayTag` _asghoability_system_component _addedgameplaytag 1)
        (set `self.AddedGameplayTag` (struct))))
    (:`CastFailed`
      (`KismetSystemLibrary.PrintString` "Remove :ASC not found")))
  (return))

(fn `SelectMovementModeGameplayTag`
  (params (Selection :type "EMovementMode Enum" :default "MOVE_None"))
  (returns (OutputPin :type "GameplayTag Structure (by ref)"))
  (return (`BlueprintGameplayTagLibrary.MakeLiteralGameplayTag` (select `EMovementMode` Selection :`MOVE_None` (struct :`TagName` "Loose.MovementMode.None") :`MOVE_Walking` (struct :`TagName` "Loose.MovementMode.Walking") :`MOVE_NavWalking` (struct :`TagName` "Loose.MovementMode.NavmeshWalking") :`MOVE_Falling` (struct :`TagName` "Loose.MovementMode.Falling") :`MOVE_Swimming` (struct :`TagName` "Loose.MovementMode.Swimming") :`MOVE_Flying` (struct :`TagName` "Loose.MovementMode.Flying") :`MOVE_Custom` (struct :`TagName` "Loose.MovementMode.Custom") :!type "GameplayTag Structure"))))