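; BP_GunProjectile is a gun projectile that applies Gameplay Ability System effects to characters it hits.
; Its lifespan derives from Range and initial speed, and it destroys itself on overlapping anything but its Instigator.
; On the server, it applies the damage and additional effect specs to an overlapped GHOCharacterBase's ASC.
; A pawn line trace toward that character recovers a hit result, which is added to the damage effect context.
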(event `self.ReceiveBeginPlay`
  (`self.SetLifeSpan` (/ (`self.Range`) (`ProjectileMovementComponent.InitialSpeed` (`self.ProjectileMovement`)))))

(event `self.Collision.OnComponentBeginOverlap`
  (params (OverlappedComponent :type "PrimitiveComponent Object Reference") (OtherActor :type "Actor Object Reference") (OtherComp :type "PrimitiveComponent Object Reference") (OtherBodyIndex :type Integer) (bFromSweep :type Boolean) (SweepResult :type "HitResult Structure (by ref)"))
  (bind _damageeffectspechandle (`self.DamageEffectSpecHandle`))
  (if (!= OtherActor (`self.GetInstigator`))
    (`/Engine/EditorBlueprintResources/ActorMacros.Switch Has Authority`
      (:`Authority`
        (bind _asghocharacter_base (cast `GHOCharacterBase` OtherActor)
          (:`then`
            (bind _returnvalue (`self.GetAbilitySystemComponent` _asghocharacter_base))
            (`/Engine/EditorBlueprintResources/StandardMacros.IsValid` _returnvalue
              (:`Is Valid`
                (bind _hitresult (`self.FindHitResult` _asghocharacter_base))
                (bind _returnvalue_2 (`AbilitySystemBlueprintLibrary.GetEffectContext` _damageeffectspechandle))
                (`AbilitySystemBlueprintLibrary.EffectContextAddHitResult` _returnvalue_2 _hitresult)
                (`AbilitySystemComponent.BP_ApplyGameplayEffectSpecToSelf` _returnvalue _damageeffectspechandle)
                (for _array_element (`self.AdditionalEffectSpecHandles`)
                  (`AbilitySystemComponent.BP_ApplyGameplayEffectSpecToSelf` _returnvalue _array_element)))
              (:`Is Not Valid`
                _)))
          (:`CastFailed`
            _)))
      (:`Remote`
        _))
    (`self.K2_DestroyActor`)))

(fn `FindHitResult`
  (params (Character :type "GHOCharacterBase Object Reference"))
  (returns (HitResult :type "HitResult Structure"))
  (bind _outhits (`KismetSystemLibrary.LineTraceMultiForObjects` (`self.K2_GetActorLocation`) (`self.K2_GetActorLocation` Character) (`|MakeArray` "ObjectTypeQuery3" :!type "EObjectTypeQuery Enum")))
  (for _array_element _outhits
    (if (== (`.HitActor` (`GameplayStatics.BreakHitResult` _array_element)) Character)
      (return _array_element)))
  (return))

(fn `GetAbilitySystemComponent`
  (params (Character :type "GHOCharacterBase Object Reference"))
  (returns (ReturnValue :type "AbilitySystemComponent Object Reference"))
  (return (`AbilitySystemBlueprintLibrary.GetAbilitySystemComponent` Character)))

(fn `UserConstructionScript`)