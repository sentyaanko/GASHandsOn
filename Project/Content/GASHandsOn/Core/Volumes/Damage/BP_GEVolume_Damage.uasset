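; BP_GEVolume_Damage is a volume Blueprint that deals damage by applying a Gameplay Effect to a given Ability System Component.
; IsValidGE reports whether the GameplayEffect class is set.
; ApplyGE builds a level 1 spec from that component, passes Damage as a SetByCaller magnitude under Data.Damage, and applies it to the same component.
; Its own event graph is inactive, so nothing here triggers the application.
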(fn `ApplyGE`
  (params (AbilitySystemComponent :type "AbilitySystemComponent Object Reference"))
  (bind _returnvalue (`AbilitySystemBlueprintLibrary.AssignTagSetByCallerMagnitude` (`AbilitySystemComponent.MakeOutgoingSpec` AbilitySystemComponent (`self.GameplayEffect`) 1.0 (`AbilitySystemComponent.MakeEffectContext` AbilitySystemComponent)) (struct :`TagName` "Data.Damage") (`self.Damage`)))
  (`AbilitySystemComponent.BP_ApplyGameplayEffectSpecToSelf` AbilitySystemComponent _returnvalue))

(fn `IsValidGE`
  (returns (ReturnValue :type Boolean))
  (return (`KismetSystemLibrary.IsValidClass` (`self.GameplayEffect`))))

(fn `UserConstructionScript`
  (`parent.UserConstructionScript`))