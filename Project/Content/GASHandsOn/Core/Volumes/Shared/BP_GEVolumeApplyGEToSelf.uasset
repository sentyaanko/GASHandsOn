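; Gameplay effect volume Blueprint that applies a configured GameplayEffect class to an Ability System Component as a self-applied effect.
; ApplyGE takes the target component, creates an effect context from it and applies the effect to that same component at a fixed level.
; IsValidGE reports whether the effect class is set.
; The event graph holds only disabled placeholders, so this file contains no overlap or trigger logic.
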(fn `ApplyGE`
  (params (AbilitySystemComponent :type "AbilitySystemComponent Object Reference"))
  (`AbilitySystemComponent.BP_ApplyGameplayEffectToSelf` AbilitySystemComponent (`self.GameplayEffect`) 1.0 (`AbilitySystemComponent.MakeEffectContext` AbilitySystemComponent)))

(fn `IsValidGE`
  (returns (ReturnValue :type Boolean))
  (return (`KismetSystemLibrary.IsValidClass` (`self.GameplayEffect`))))

(fn `UserConstructionScript`
  (`parent.UserConstructionScript`))