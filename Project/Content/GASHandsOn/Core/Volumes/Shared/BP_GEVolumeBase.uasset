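; Base volume actor that periodically applies a Gameplay Effect to living GHOCharacterBase characters overlapping its Box.
; On BeginPlay, a passing IsValidGE check starts a looping one-second timer, which is cleared on Destroyed.
; Each tick runs on authority only, finds each character's Ability System Component and passes it to ApplyGE.
; IsValidGE returns false and ApplyGE is empty, leaving both for subclasses; the construction script sets label text and color.
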(event `self.ReceiveBeginPlay`
  (bind _returnvalue (`self.IsValidGE`))
  (if _returnvalue
    (bind _returnvalue_2 (`KismetSystemLibrary.K2_SetTimerDelegate` (delegate `ApplyGameplayEffectTick`) 1.0 true))
    (set `self.TimerHandle` _returnvalue_2)))

(event `ApplyGameplayEffectTick`
  (`/Engine/EditorBlueprintResources/ActorMacros.Switch Has Authority`
    (:`Authority`
      (for _array_element (`PrimitiveComponent.GetOverlappingActors` (`self.Box`) "/Script/GASHandsOn.GHOCharacterBase")
        (bind _asghocharacter_base (cast `GHOCharacterBase` _array_element))
        (if (`GHOCharacterBase.IsAlive` _asghocharacter_base)
          (bind _returnvalue (`self.GetAbilitySystemComponent` _asghocharacter_base))
          (`/Engine/EditorBlueprintResources/StandardMacros.IsValid` _returnvalue
            (:`Is Valid`
              (`self.ApplyGE` _returnvalue))))))))

(event `self.ReceiveDestroyed`
  (`KismetSystemLibrary.K2_ClearAndInvalidateTimerHandle` (`self.TimerHandle`)))

(fn `ApplyGE`
  (params (AbilitySystemComponent :type "AbilitySystemComponent Object Reference")))

(fn `GetAbilitySystemComponent`
  (params (Actor :type "Actor Object Reference"))
  (returns (ReturnValue :type "AbilitySystemComponent Object Reference"))
  (return (`AbilitySystemBlueprintLibrary.GetAbilitySystemComponent` Actor)))

(fn `IsValidGE`
  (returns (ReturnValue :type Boolean))
  (return false))

(fn `UserConstructionScript`
  (bind _textrender (`self.TextRender`))
  (`TextRenderComponent.K2_SetText` _textrender (`self.Text`))
  (`TextRenderComponent.SetTextRenderColor` _textrender (`self.TextColor`)))