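; Rifle secondary Gameplay Ability that aims down sights while input is held.
; Activation applies an aiming effect, tweens camera FOV, sets boom length and starts movement-component ADS, then calls empty lock-on trace hooks.
; Release zooms back and applies a removal effect whose tag predicts the ADS stop, ending once FOV is restored.
; Ending also covers external cancels by ensuring that effect applies before clearing effects, tasks, camera and movement state.
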(event `self.K2_ActivateAbility`
  (bind (_returnvalue_owneractor _returnvalue_avataractor _returnvalue_playercontroller _returnvalue_abilitysystemcomponent _returnvalue_skeletalmeshcomponent _returnvalue_animinstance _returnvalue_movementcomponent) (break `GameplayAbilityActorInfo` (`self.GetActorInfo`)))
  (bind _owninghero (`self.OwningHero`))
  (set `self.GE_AimingRemoval` (struct))
  (bind _success (`self.CheckAndSetUpCacheables`))
  (if _success
    (bind _returnvalue (`self.BP_ApplyGameplayEffectToOwner` (`self.GE_AimingClass`) (`self.GetAbilityLevel`)))
    (set `self.GE_Aiming` _returnvalue)
    ;[1 1 1] zoom in
    (bind _asynctaskproxy (`GHOAbilityTask_WaitChangeFOV.WaitChangeFOV` "None" (`GHOHeroCharacterBase.FollowCamera` _owninghero) (`self.TargetingFOV`) (`self.ZoomInDuration`))
      (:`then`
        (set `self.ZoomInAsyncTask` _asynctaskproxy)
        (set `SpringArmComponent.TargetArmLength` (`self.TargetArmLengthDuringZoomIn`) (`GHOHeroCharacterBase.CameraBoom` _owninghero))
        (bind _asghocharacter_movement_component (cast `GHOCharacterMovementComponent` _returnvalue_movementcomponent))
        (`GHOCharacterMovementComponent.StartAimDownSights` _asghocharacter_movement_component)
        (`AbilityTask_WaitInputRelease.WaitInputRelease` true
          (:`then`
            (`self.BeginRockOnTrace`))
          (:`OnRelease`
            (`self.ZoomBack`)))))))

(event `ZoomBack`
  (bind _owninghero (`self.OwningHero`))
  ;[1 1 1] zoom back
  (bind _asynctaskproxy (`GHOAbilityTask_WaitChangeFOV.WaitChangeFOV` "None" (`GHOHeroCharacterBase.FollowCamera` _owninghero) (`GHOHeroCharacterBase.DefaultFOV` _owninghero) (`self.ZoomBackDuration`))
    (:`then`
      (set `self.ZoomBackAsyncTask` _asynctaskproxy)
      (`self.ApplyAimingRemovalEffect`))
    (:`OnTargetFOVReached`
      (`self.K2_EndAbility`))))

(event `self.K2_OnEndAbility`
  (params (bWasCancelled :type Boolean))
  (bind (_returnvalue_owneractor _returnvalue_avataractor _returnvalue_playercontroller _returnvalue_abilitysystemcomponent _returnvalue_skeletalmeshcomponent _returnvalue_animinstance _returnvalue_movementcomponent) (break `GameplayAbilityActorInfo` (`self.GetActorInfo`)))
  (bind _owninghero (`self.OwningHero`))
  (`self.EndRockOnTrace`)
  ;[1 1 1] Apply the removal GameplayEffect's GameplayTag to predict stopping AimDownSights
  ; if we didn't do it naturally by releasing input (external cancel).
  (bind _returnvalue (`AbilitySystemBlueprintLibrary.GetActiveGameplayEffectStackCount` (`self.GE_AimingRemoval`)))
  (if (not (> _returnvalue 0))
    (`self.ApplyAimingRemovalEffect`))
  (`self.BP_RemoveGameplayEffectFromOwnerWithHandle` (`self.GE_Aiming`))
  (`self.BP_RemoveGameplayEffectFromOwnerWithHandle` (`self.GE_AimingRemoval`))
  ;[1 1 1] Kill tasks in case ability was ended before they finished
  (bind _zoominasynctask (`self.ZoomInAsyncTask`)
    (:`then`
      (`GameplayTask.EndTask` _zoominasynctask))
    (:`else`
      _))
  (bind _zoombackasynctask (`self.ZoomBackAsyncTask`)
    (:`then`
      (`GameplayTask.EndTask` _zoombackasynctask))
    (:`else`
      _))
  ;[1 1 1] zoom reset
  (`CameraComponent.SetFieldOfView` (`GHOHeroCharacterBase.FollowCamera` _owninghero) (`GHOHeroCharacterBase.DefaultFOV` _owninghero))
  (set `SpringArmComponent.TargetArmLength` (`GHOHeroCharacterBase.StartingCameraBoomTargetArmLength` _owninghero) (`GHOHeroCharacterBase.CameraBoom` _owninghero))
  (bind _asghocharacter_movement_component (cast `GHOCharacterMovementComponent` _returnvalue_movementcomponent))
  (`GHOCharacterMovementComponent.StopAimDownSights` _asghocharacter_movement_component))

(event `BeginRockOnTrace`)

(event `EndRockOnTrace`)

(fn `ApplyAimingRemovalEffect`
  (bind _returnvalue (`self.BP_ApplyGameplayEffectToOwner` (`self.GE_AimingRemovalClass`) (`self.GetAbilityLevel`)))
  (set `self.GE_AimingRemoval` _returnvalue)
  (return))

(fn `CheckAndSetUpCacheables`
  (returns (Success :type Boolean))
  (`self.OwningHero`
    (:`then`
      _)
    (:`else`
      (bind _asghohero_character_base (cast `GHOHeroCharacterBase` (`self.GetAvatarActorFromActorInfo`))
        (:`then`
          (set `self.OwningHero` _asghohero_character_base))
        (:`CastFailed`
          (return false)))))
  (return true))