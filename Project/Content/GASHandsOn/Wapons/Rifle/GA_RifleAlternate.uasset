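; Gameplay ability for the rifle's alternate action that cycles the weapon to its next fire mode.
; On activation it caches the source weapon and, if one exists, the player controller, since AI has none.
; It advances through the FireModes list with wraparound, sets the matching status text on the weapon, pushes it to the player controller's display, then ends.
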(event `self.K2_ActivateAbility`
  (bind (_returnvalue_owneractor _returnvalue_avataractor _returnvalue_playercontroller) (break `GameplayAbilityActorInfo` (`self.GetActorInfo`)))
  (bind _firemodes (`self.FireModes`))
  (bind _weapon (`self.Weapon`))
  (bind _returnvalue (`KismetArrayLibrary.Array_Find` _firemodes (`GHOWeapon.FireMode` _weapon)))
  (`self.Weapon`
    (:`then`
      ;[1 1 1] Cache player controller. AI won't have one.
      (`self.PlayerContriller` :!label _label
        (:`then`
          _)
        (:`else`
          (bind _asghoplayer_controller (cast `GHOPlayerController` _returnvalue_playercontroller)
            (:`then`
              (set `self.PlayerContriller` _asghoplayer_controller))
            (:`CastFailed`
              _))))
      (if (>= _returnvalue 0)
        (bind _output_get (set `self.NextIndex` (`self.CalcNextIndex` _returnvalue (`KismetArrayLibrary.Array_Length` _firemodes))))
        (set `GHOWeapon.FireMode` (`|GetArrayItem` _firemodes _output_get) _weapon)
        (bind _output_get_2 (set `GHOWeapon.StatusText` (`|GetArrayItem` (`self.StatusTexts`) _output_get) _weapon))
        (bind _playercontriller (`self.PlayerContriller`)
          (:`then`
            (`GHOPlayerController.SetEquippedWeaponStatusText` _playercontriller _output_get_2))
          (:`else`
            _))))
    (:`else`
      (bind _asghoweapon (cast `GHOWeapon` (`self.GetCurrentSourceObject`))
        (:`then`
          (set `self.Weapon` _asghoweapon)
          (goto _label))
        (:`CastFailed`
          _))))
  (`self.K2_EndAbility`))

(fn `CalcNextIndex`
  (params (CurrentIndex :type Integer) (Length :type Integer))
  (returns (NextIndex :type Integer))
  (bind _returnvalue (+ CurrentIndex 1))
  (return (`KismetMathLibrary.SelectInt` 0 _returnvalue (== _returnvalue Length))))