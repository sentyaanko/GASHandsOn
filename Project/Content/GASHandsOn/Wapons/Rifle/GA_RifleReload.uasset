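; Gameplay Ability that reloads the rifle, allowed only when the hero's clip is not full and reserve ammo remains.
; It plays the reload montage and, on its event, uses a server-wait net sync to get a new prediction key for predicted ammo changes.
; A SetByCaller effect container deducts the available amount from reserve, and the cached source weapon's clip is increased directly.
; Montage completion ends the ability after client and server sync, while interruption cancels it.
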(event `self.K2_ActivateAbility`
  (bind _sourceweapon (`self.SourceWeapon`))
  (bind _returnvalue (`GHOWeapon.GetPrimaryClipAmmo` _sourceweapon))
  (`self.CheckAndSetUpCacheables`)
  ;[1 1 1] AvatarActor が 1pv/3pv で別の Mesh を持っているならば、
  ; PlayMontageForMeshAndWaitForEvent を使用する。
  (`GHOAbilityTask_PlayMontageAndWaitForEvent.PlayMontageAndWaitForEvent` "None" "/Game/GASHandsOn/Core/Characters/Heroes/Animations/AM_Hero_RifleReload.AM_Hero_RifleReload" (struct :`GameplayTags` (struct :`(TagName` "Ability.Weapon.Reload"))) 1.0 "None" false
    (:`OnCompleted`
      ;[1 1 1] Since we have Server respect remote cancelled enabled (so local only primary ability can cancel it), we need to sync up so that the client doesn't end before the server's montage hits the event.
      (`AbilityTask_NetworkSyncPoint.WaitNetSync` "BothWait"
        (:`OnSync`
          (`self.K2_EndAbility`))))
    (:`OnInterrupted`
      (`self.K2_CancelAbility` :!label _label))
    (:`OnCancelled`
      (goto _label))
    (:`EventReceived`
      (`AbilityTask_NetworkSyncPoint.WaitNetSync` "OnlyServerWait" ; Get a new scoped prediction key to apply the ammo changes predictively\n弾薬の変更を predictively （予測）して適用するために、新しい scoped prediction key （スコープ付き予測キー）を取得する
        (:`OnSync`
          (bind _output_get (set `self.AmountWeWantToReload` (- (`GHOWeapon.GetMaxPrimaryClipAmmo` _sourceweapon) _returnvalue)))
          (bind _output_get_2 (set `self.AmountWeCanReload` (`KismetMathLibrary.Min` _output_get (`GHOHeroCharacterBase.GetPrimaryReserveAmmo` (`self.OwningHero`)))))
          (bind _returnvalue_2 (`self.MakeEffectContainerSpec` (struct :`TagName` "Ability")))
          (`AbilitySystemBlueprintLibrary.AssignTagSetByCallerMagnitude` (`|GetArrayItem` (`.TargetGameplayEffectSpecs` (break `GHOGameplayEffectContainerSpec` _returnvalue_2))) (struct :`TagName` "Data.ReloadAmount.Reserve") (`KismetMathLibrary.Conv_IntToDouble` (* _output_get_2 -1)))
          (`self.ApplyEffectContainerSpec` _returnvalue_2)
          (`GHOWeapon.SetPrimaryClipAmmo` _sourceweapon (+ _output_get_2 _returnvalue)))))))

(fn `K2_CanActivateAbility`
  (params (ActorInfo :type "GameplayAbilityActorInfo Structure"))
  (returns (RelevantTags :type "GameplayTagContainer Structure") (ReturnValue :type Boolean))
  (bind _asbp_hero_character_base (cast `/Game/GASHandsOn/Core/Characters/Heroes/BP_HeroCharacterBase` (`.AvatarActor` (break `GameplayAbilityActorInfo` ActorInfo)))
    (:`then`
      (return (struct) (and (< (`GHOHeroCharacterBase.GetPrimaryClipAmmo` _asbp_hero_character_base) (`GHOHeroCharacterBase.GetMaxPrimaryClipAmmo` _asbp_hero_character_base)) (> (`GHOHeroCharacterBase.GetPrimaryReserveAmmo` _asbp_hero_character_base) 0))))
    (:`CastFailed`
      (return (struct) false))))