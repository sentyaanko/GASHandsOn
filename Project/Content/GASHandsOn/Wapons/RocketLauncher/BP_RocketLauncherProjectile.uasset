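; Rocket launcher projectile that can home on a target and deals area damage on overlap.
; On authority, overlapping a non-instigator triggers a sphere trace for living characters, applies the damage effect container to them and destroys the rocket; remotes just destroy it.
; Fire and impact effects run as local GameplayCues on the first player's ability system, since an AI shooter's may be gone.
; Locally controlled shooters skip the fire cue.
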(event `self.ReceiveBeginPlay`
  (bind _asghohero_character_base (cast `GHOHeroCharacterBase` (`self.GetInstigator`)))
  ;[1 1 1] Use the local player's ASC since we can't guarantee AI ASC's will still exist if they die after firing the rocket.
  (bind _asghoability_system_component (cast `GHOAbilitySystemComponent` (`AbilitySystemBlueprintLibrary.GetAbilitySystemComponent` (`Controller.PlayerState` (`GameplayStatics.GetPlayerController` 0)))))
  (bind _output_get (set `self.ASC` _asghoability_system_component))
  ;[1 1 1] Muzzle FX will play for locally controlled player on the Instant Ability
  (if (not (`Pawn.IsLocallyControlled` _asghohero_character_base))
    (`GHOAbilitySystemComponent.ExecuteGameplayCueLocal` _output_get (struct :`TagName` "GameplayCue.Weapon.RocketLauncher.Fire") (`AbilitySystemBlueprintLibrary.MakeGameplayCueParameters` 0.0 0.0 (struct) (struct) (struct) (struct) (struct) (`self.K2_GetActorLocation`) (`KismetMathLibrary.GetForwardVector` (`self.K2_GetActorRotation`)) _asghohero_character_base))))

(event `self.Sphere.OnComponentBeginOverlap`
  (params (OverlappedComponent :type "PrimitiveComponent Object Reference") (OtherActor :type "Actor Object Reference") (OtherComp :type "PrimitiveComponent Object Reference") (OtherBodyIndex :type Integer) (bFromSweep :type Boolean) (SweepResult :type "HitResult Structure (by ref)"))
  (bind _returnvalue (`self.K2_GetActorLocation`))
  (bind _damageeffectcontainerspec (`self.DamageEffectContainerSpec`))
  (bind _hittargets (`self.HitTargets`))
  (`KismetSystemLibrary.PrintString` "Hello")
  (`/Engine/EditorBlueprintResources/ActorMacros.Switch Has Authority`
    (:`Authority`
      (if (!= (`self.GetInstigator`) OtherActor)
        (bind _outhits (`KismetSystemLibrary.SphereTraceMultiForObjects` _returnvalue (+ _returnvalue 0.01) (`self.ExplosionRadius`) (`|MakeArray` "ObjectTypeQuery3" :!type "EObjectTypeQuery Enum")))
        (for _array_element _outhits
          (bind _asghocharacter_base (cast `GHOCharacterBase` (`.HitActor` (`GameplayStatics.BreakHitResult` _array_element))))
          (if (`GHOCharacterBase.IsAlive` _asghocharacter_base)
            (`KismetArrayLibrary.Array_AddUnique` (`self.HitTargets`) _asghocharacter_base)))
        (if (!= (`KismetArrayLibrary.Array_Length` _hittargets) 0)
          (`GHOBlueprintFunctionLibrary.AddTargetsToEffectContainerSpec` :`ContainerSpec` _damageeffectcontainerspec :`TargetActors` _hittargets)
          (`GHOBlueprintFunctionLibrary.ApplyExternalEffectContainerSpec` _damageeffectcontainerspec))
        (`self.K2_DestroyActor`)))
    (:`Remote`
      (`self.K2_DestroyActor`))))

(event `self.ReceiveEndPlay`
  (params (EndPlayReason :type "EEndPlayReason Enum" :default "Destroyed"))
  (bind _asc (`self.ASC`)
    (:`then`
      (`GHOAbilitySystemComponent.ExecuteGameplayCueLocal` _asc (struct :`TagName` "GameplayCue.Weapon.RocketLauncher.Impact") (`AbilitySystemBlueprintLibrary.MakeGameplayCueParameters` 0.0 0.0 (struct) (struct) (struct) (struct) (struct) (`self.K2_GetActorLocation`))))
    (:`else`)))

(fn `UserConstructionScript`
  (bind _projectilemovement (`self.ProjectileMovement`))
  (set `ProjectileMovementComponent.bIsHomingProjectile` (`self.IsHoming`) _projectilemovement)
  (bind _homingtarget (`self.HomingTarget`)
    (:`then`
      (set `ProjectileMovementComponent.HomingTargetComponent` (`Actor.RootComponent` _homingtarget) _projectilemovement))
    (:`else`)))