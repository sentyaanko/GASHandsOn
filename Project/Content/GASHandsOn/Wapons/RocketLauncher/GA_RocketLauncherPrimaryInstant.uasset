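; Gameplay ability for the rocket launcher's instant primary fire, launching a rocket from received target data.
; HandleTargetData commits the ability cost, cancelling the ability if that fails.
; The server spawns the projectile aimed from trace start to hit location, passing it a damage effect container with SetByCaller bullet damage.
; The locally controlled player runs the fire GameplayCue locally for immediate feedback.
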(event `self.HandleTargetData`
  (params (TargetData :type "GameplayAbilityTargetDataHandle Structure"))
  (bind (_bblockinghit _binitialoverlap _time _distance _location _impactpoint _normal _impactnormal _physmat _hitactor _hitcomponent _hitbonename _hititem _faceindex _tracestart) (`GameplayStatics.BreakHitResult` (`AbilitySystemBlueprintLibrary.GetHitResultFromTargetData` TargetData)))
  (bind _returnvalue (`KismetMathLibrary.FindLookAtRotation` _tracestart _location))
  ;[1 1 1] Handle a fired rocket (Server receives the TargetData or client fires a rocket).
  (bind _returnvalue_2 (`self.K2_CommitAbilityCost` false))
  (if _returnvalue_2
    (if (`Actor.HasAuthority` (`self.OwningHero`))
      (bind _returnvalue_3 (`self.MakeEffectContainerSpec` (struct :`TagName` "Ability")))
      (`AbilitySystemBlueprintLibrary.AssignTagSetByCallerMagnitude` (`|GetArrayItem` (`.TargetGameplayEffectSpecs` (break `GHOGameplayEffectContainerSpec` _returnvalue_3))) (struct :`TagName` "Data.Damage") (`self.BulletDamage`))
      (`|SpawnActorFromClass` :`Class` "/Game/GASHandsOn/Wapons/RocketLauncher/BP_RocketLauncherProjectile.BP_RocketLauncherProjectile_C" :`SpawnTransform` (`KismetMathLibrary.MakeTransform` _tracestart _returnvalue) :`CollisionHandlingOverride` "AlwaysSpawn" :`TransformScaleMethod` "OverrideRootScale" :`HomingTarget` null :`DamageEffectContainerSpec` _returnvalue_3 :`Instigator` (`self.OwningHero`)))
    ;[1 1 1] Play Fire FX immediately for locally controlled player
    (if (`Pawn.IsLocallyControlled` (`self.OwningHero`))
      (bind _asghoability_system_component (cast `GHOAbilitySystemComponent` (`self.GetAbilitySystemComponentFromActorInfo`)))
      (`GHOAbilitySystemComponent.ExecuteGameplayCueLocal` _asghoability_system_component (struct :`TagName` "GameplayCue.Weapon.RocketLauncher.Fire") (`AbilitySystemBlueprintLibrary.MakeGameplayCueParameters` 0.0 0.0 (struct) (struct) (struct) (struct) (struct) _location (`KismetMathLibrary.GetForwardVector` _returnvalue) (`self.OwningHero`))))
    (else
      (`self.K2_CancelAbility`))))