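; BP_Door is an interactable sliding door whose open state is driven by a Gameplay Ability System tag.
; Interacting with its Button makes the server toggle GE_DoorOpen on the door's own ability system component.
; An async tag listener calls MoveDoor whenever ListenTag is added or removed, and ends on EndPlay.
; A timeline slides the door along local Y, offsetting its start time by current position to handle mid-motion reversals.
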(event `self.ReceiveBeginPlay`
  (bind _listentag (`self.ListenTag`))
  (bind (_asynctaskproxy _tag) (`GHOAsyncTaskGameplayTagAddedRemoved.ListenForGameplayTagAddedOrRemoved` (`AbilitySystemBlueprintLibrary.GetAbilitySystemComponent` self) (`BlueprintGameplayTagLibrary.MakeGameplayTagContainerFromArray` (`|MakeArray` _listentag)))
    (:`then`
      (set `self.ListenForGameplayTagAddedOrRemovedAsyncTask` _asynctaskproxy))
    (:`OnTagAdded`
      (bind _returnvalue (== _tag _listentag))
      (if _returnvalue
        (`self.MoveDoor` true)))
    (:`OnTagRemoved`
      (if _returnvalue
        (`self.MoveDoor` false)))))

(event `self.PostInteract`
  (params (InteractingActor :type "Actor Object Reference") (InteractionComponent :type "PrimitiveComponent Object Reference"))
  (bind _returnvalue (`AbilitySystemBlueprintLibrary.GetAbilitySystemComponent` self))
  (if (== InteractionComponent (`self.Button`))
    (`/Engine/EditorBlueprintResources/ActorMacros.Switch Has Authority`
      (:`Authority`
        (if (`GameplayTagAssetInterface.HasMatchingGameplayTag` _returnvalue (`self.ListenTag`))
          (`AbilitySystemComponent.RemoveActiveGameplayEffect` _returnvalue (`self.GE_DoorOpen`) -1)
          (else
            (bind _returnvalue_2 (`AbilitySystemComponent.BP_ApplyGameplayEffectToSelf` _returnvalue "/Game/GASHandsOn/Environments/Door/GE_DoorOpen.GE_DoorOpen_C" 0.0 (`AbilitySystemComponent.MakeEffectContext` _returnvalue)))
            (set `self.GE_DoorOpen` _returnvalue_2)))))))

(event `MoveDoor`
  (params (bIsOpen :type Boolean))
  (bind _startingtime (`self.StartingTime`))
  (bind _maxdoormovementdistance (`self.MaxDoorMovementDistance`))
  (bind (_relativelocation_x _relativelocation_y) (`KismetMathLibrary.BreakVector` (`SceneComponent.RelativeLocation` (`self.Door`))))
  (`TimelineComponent.Stop` (`self.DoorTimeline`))
  (bind _output_get (set `self.DoorStartingRelativeLocationY` _relativelocation_y))
  (set `self.DoorTargetRelativeLocationY` (`KismetMathLibrary.SelectFloat` _maxdoormovementdistance 0.0 bIsOpen))
  (bind _returnvalue (/ _output_get _maxdoormovementdistance))
  (bind _output_get_2 (set `self.StartingTime` (* (`KismetMathLibrary.SelectFloat` _returnvalue (- 1.0 _returnvalue) bIsOpen) (`self.TimeToOpenCloseDoor`))))
  (`|ExecutionSequence`
    (:`then_0`
      (bind (_direction _time) (`Timeline|DoorTimeline` :`NewTime` _output_get_2 :!via `SetNewTime` :!label _label)
        (:`Update`
          (`SceneComponent.K2_SetRelativeLocation` (`self.Door`) (`KismetMathLibrary.MakeVector` 0.0 (`KismetMathLibrary.Lerp` (`self.DoorStartingRelativeLocationY`) (`self.DoorTargetRelativeLocationY`) (/ (- _time _startingtime) (- (`self.TimeToOpenCloseDoor`) _startingtime)))) false false))))
    (:`then_1`
      (goto _label))))

(event `self.ReceiveEndPlay`
  (params (EndPlayReason :type "EEndPlayReason Enum" :default "Destroyed"))
  (bind _listenforgameplaytagaddedorremovedasynctask (`self.ListenForGameplayTagAddedOrRemovedAsyncTask`)
    (:`then`
      (`GHOAsyncTaskGameplayTagAddedRemoved.EndTask` _listenforgameplaytagaddedorremovedasynctask))
    (:`else`)))

(fn `GetInteractionDuration`
  (params (InteractionComponent :type "PrimitiveComponent Object Reference"))
  (returns (ReturnValue :type "Float (double-precision)"))
  (return 0.0))

(fn `GetPostInteractSyncType`
  (params (InteractionComponent :type "PrimitiveComponent Object Reference"))
  (returns (bShouldSync :type Boolean) (Type :type "EAbilityTaskNetSyncType Enum"))
  (return false "BothWait"))

(fn `GetPreInteractSyncType`
  (params (InteractionComponent :type "PrimitiveComponent Object Reference"))
  (returns (bShouldSync :type Boolean) (Type :type "EAbilityTaskNetSyncType Enum"))
  (return false "BothWait"))

(fn `IsAvailableForInteraction`
  (params (InteractionComponent :type "PrimitiveComponent Object Reference"))
  (returns (ReturnValue :type Boolean))
  (return (== InteractionComponent (`self.Button`))))

(fn `UserConstructionScript`)