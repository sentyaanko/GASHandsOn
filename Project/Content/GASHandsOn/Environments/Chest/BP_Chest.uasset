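; Interactable chest that uses the Gameplay Ability System to open, close and spawn loot.
; Interacting with the lock applies an interacting effect on the server, then on completion an open effect and spawns a random weapon and item on an elliptical arc around it.
; An async gameplay tag listener animates the lid with RotatingMovement and drops or restores the lock.
; Tags on the chest gate availability.
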(event `self.ReceiveBeginPlay`
  (bind _listentag (`self.ListenTag`))
  (`MovementComponent.SetUpdatedComponent` (`self.RotatingMovement`) (`self.SM_ChestTop`))
  (bind (_asynctaskproxy _tag) (`GHOAsyncTaskGameplayTagAddedRemoved.ListenForGameplayTagAddedOrRemoved` (`AbilitySystemBlueprintLibrary.GetAbilitySystemComponent` self) (`BlueprintGameplayTagLibrary.MakeGameplayTagContainerFromTag` _listentag))
    (:`then`
      (set `self.ListenForGameplayTagAddedOrRemovedAsyncTask` _asynctaskproxy)
      (set `self.LockStartingRelativeLocation` (`SceneComponent.RelativeLocation` (`self.SM_ChestLock`))))
    (:`OnTagAdded`
      (bind _returnvalue (== _tag _listentag))
      (if _returnvalue
        (`self.OpenChest`)))
    (:`OnTagRemoved`
      (if _returnvalue
        (`self.CloseChest`)))))

(event `self.PreInteract`
  (params (InteractingActor :type "Actor Object Reference") (InteractionComponent :type "PrimitiveComponent Object Reference"))
  (bind _returnvalue (`AbilitySystemBlueprintLibrary.GetAbilitySystemComponent` self))
  (if (== InteractionComponent (`self.SM_ChestLock`))
    (`/Engine/EditorBlueprintResources/ActorMacros.Switch Has Authority`
      (:`Authority`
        (bind _returnvalue_2 (`AbilitySystemComponent.BP_ApplyGameplayEffectToSelf` _returnvalue "/Game/GASHandsOn/Core/Characters/Shared/Abilities/Interact/GE_Interacting.GE_Interacting_C" 0.0 (`AbilitySystemComponent.MakeEffectContext` _returnvalue)))
        (set `self.GE_InteractingHandle` _returnvalue_2)))))

(event `self.PostInteract`
  (params (InteractingActor :type "Actor Object Reference") (InteractionComponent :type "PrimitiveComponent Object Reference"))
  (bind _returnvalue (`AbilitySystemBlueprintLibrary.GetAbilitySystemComponent` InteractingActor))
  (bind _returnvalue_2 (`AbilitySystemBlueprintLibrary.GetAbilitySystemComponent` self))
  (if (== InteractionComponent (`self.SM_ChestLock`))
    (`/Engine/EditorBlueprintResources/ActorMacros.Switch Has Authority`
      (:`Authority`
        (`AbilitySystemComponent.BP_ApplyGameplayEffectToTarget` _returnvalue "/Game/GASHandsOn/Environments/Chest/GE_ChestOpen.GE_ChestOpen_C" _returnvalue_2 0.0 (`AbilitySystemComponent.MakeEffectContext` _returnvalue))
        (`AbilitySystemComponent.RemoveActiveGameplayEffect` _returnvalue_2 (`self.GE_InteractingHandle`) -1)
        (for _array_element (`|MakeArray` (`KismetArrayLibrary.Array_Random` (`self.WeaponClasses`)) (`KismetArrayLibrary.Array_Random` (`self.ItemClasses`)) :!type "Actor Class Reference")
          (bind _returnvalue_3 (`self.GetLocationToSpawnItem`))
          (`|SpawnActorFromClass` _array_element (`KismetMathLibrary.MakeTransform` _returnvalue_3 (`self.K2_GetActorRotation`)) "Undefined" "OverrideRootScale" null null))))))

(event `OpenChest`
  (bind _rotatingmovement (`self.RotatingMovement`))
  (bind _sm_chestlock (`self.SM_ChestLock`))
  (bind (_lockstartingrelativelocation_x _lockstartingrelativelocation_y _lockstartingrelativelocation_z) (`KismetMathLibrary.BreakVector` (`self.LockStartingRelativeLocation`)))
  (set `RotatingMovementComponent.RotationRate` (struct :`Pitch` 180.0) _rotatingmovement)
  (`ActorComponent.Activate` _rotatingmovement true)
  (`|ExecutionSequence`
    (:`then_0`
      (`KismetSystemLibrary.Delay` (`self.ChestTopAnimationDuration`))
      (`MovementComponent.StopMovementImmediately` _rotatingmovement)
      (`ActorComponent.Deactivate` _rotatingmovement))
    (:`then_1`
      (bind (_direction _time) (`Timeline|LockFallOff` :!via `PlayFromStart`)
        (:`Update`
          (`SceneComponent.K2_SetRelativeLocation` _sm_chestlock (`KismetMathLibrary.MakeVector` _lockstartingrelativelocation_x _lockstartingrelativelocation_y (+ _lockstartingrelativelocation_z (`KismetMathLibrary.Lerp` 0.0 (`self.LockFallOffRelativeLocationZ`) (/ _time (`self.ChestTopAnimationDuration`))))) false false))
        (:`Finished`
          (`SceneComponent.SetVisibility` _sm_chestlock false true))))))

(event `CloseChest`
  (bind _rotatingmovement (`self.RotatingMovement`))
  (bind _sm_chestlock (`self.SM_ChestLock`))
  (set `RotatingMovementComponent.RotationRate` (struct :`Pitch` -180.0) _rotatingmovement)
  (`ActorComponent.Activate` _rotatingmovement true)
  (`KismetSystemLibrary.Delay` (`self.ChestTopAnimationDuration`))
  (`MovementComponent.StopMovementImmediately` _rotatingmovement)
  (`ActorComponent.Deactivate` _rotatingmovement)
  (`SceneComponent.SetVisibility` _sm_chestlock true true)
  (`SceneComponent.K2_SetRelativeLocation` _sm_chestlock (`self.LockStartingRelativeLocation`) false false))

(event `self.ReceiveEndPlay`
  (params (EndPlayReason :type "EEndPlayReason Enum" :default "Destroyed"))
  (bind _listenforgameplaytagaddedorremovedasynctask (`self.ListenForGameplayTagAddedOrRemovedAsyncTask`)
    (:`then`
      (`GHOAsyncTaskGameplayTagAddedRemoved.EndTask` _listenforgameplaytagaddedorremovedasynctask))
    (:`else`)))

(event `self.CancelInteraction`
  (params (InteractionComponent :type "PrimitiveComponent Object Reference"))
  (if (== InteractionComponent (`self.SM_ChestLock`))
    (`AbilitySystemComponent.RemoveActiveGameplayEffect` (`AbilitySystemBlueprintLibrary.GetAbilitySystemComponent` self) (`self.GE_InteractingHandle`) -1)))

(fn `GetInteractionDuration`
  (params (InteractionComponent :type "PrimitiveComponent Object Reference"))
  (returns (ReturnValue :type "Float (double-precision)"))
  (return (`KismetMathLibrary.SelectFloat` (`self.OpenChestDuration`) 0.0 (== InteractionComponent (`self.SM_ChestLock`)))))

(fn `GetLocationToSpawnItem`
  (returns (ReturnValue :type "Vector Structure"))
  (locals (Degree :type "Float (double-precision)" :default 0.0) (EllipseXRadius :type "Float (double-precision)" :default 100.0) (EllipseYRadius :type "Float (double-precision)" :default 150.0))
  (bind (_returnvalue_roll _returnvalue_pitch _returnvalue_yaw) (`KismetMathLibrary.BreakRotator` (`self.K2_GetActorRotation`)))
  (bind _output_get (set `local.Degree` (`KismetMathLibrary.RandomFloatInRange` -90.0 90.0)))
  (return (+ (`self.K2_GetActorLocation`) (`KismetMathLibrary.GreaterGreater_VectorRotator` (`KismetMathLibrary.MakeVector` (* (`local.EllipseXRadius`) (`KismetMathLibrary.DegCos` _output_get)) (* (`local.EllipseYRadius`) (`KismetMathLibrary.DegSin` _output_get))) (`KismetMathLibrary.MakeRotator` 0.0 0.0 _returnvalue_yaw)) (0.0 0.0 100.0))))

(fn `GetPostInteractSyncType`
  (params (InteractionComponent :type "PrimitiveComponent Object Reference"))
  (returns (bShouldSync :type Boolean) (Type :type "EAbilityTaskNetSyncType Enum"))
  (return false "OnlyServerWait"))

(fn `GetPreInteractSyncType`
  (params (InteractionComponent :type "PrimitiveComponent Object Reference"))
  (returns (bShouldSync :type Boolean) (Type :type "EAbilityTaskNetSyncType Enum"))
  (bind _returnvalue (== InteractionComponent (`self.SM_ChestLock`)))
  (return _returnvalue (select `bool` _returnvalue :`false` "BothWait" :`true` "OnlyClientWait" :!type "EAbilityTaskNetSyncType Enum")))

(fn `IsAvailableForInteraction`
  (params (InteractionComponent :type "PrimitiveComponent Object Reference"))
  (returns (ReturnValue :type Boolean))
  (if (== InteractionComponent (`self.SM_ChestLock`))
    (return (not (`GameplayTagAssetInterface.HasAnyMatchingGameplayTags` (`AbilitySystemBlueprintLibrary.GetAbilitySystemComponent` self) (`self.AvailabilityTags`))))
    (else
      (return false))))

(fn `UserConstructionScript`)