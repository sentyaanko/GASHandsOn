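; Bullet ammo pickup Blueprint that extends a parent pickup with an eligibility check and particle feedback.
; CanBePickedUp requires the parent check to pass, then compares two float attributes from the character's Ability System Component, allowing pickup only while the first is below the second.
; OnPickedUp and OnRespawned call the parent, then deactivate or reactivate the PSPickupAmmoBullet effect respectively.
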(event `self.OnPickedUp`
  (`parent.OnPickedUp`)
  (`ActorComponent.Deactivate` (`self.PS_Pickup_AmmoBullet`)))

(event `self.OnRespawned`
  (`parent.OnRespawned`)
  (`ActorComponent.Activate` (`self.PS_Pickup_AmmoBullet`) true))

(fn `CanBePickedUp`
  (params (TestCharacter :type "GHOCharacterBase Object Reference"))
  (returns (ReturnValue :type Boolean))
  (bind _returnvalue (`AbilitySystemBlueprintLibrary.GetAbilitySystemComponent` TestCharacter))
  (bind _returnvalue_2 (`parent.CanBePickedUp` TestCharacter))
  (if _returnvalue_2
    (return (< (`.ReturnValue` (`AbilitySystemBlueprintLibrary.GetFloatAttributeFromAbilitySystemComponent` _returnvalue (struct :`AttributeName` "RifleReserveAmmo" :`Attribute` "/Script/GASHandsOn.GHOAttributeSetAmmo:RifleReserveAmmo"))) (`.ReturnValue` (`AbilitySystemBlueprintLibrary.GetFloatAttributeFromAbilitySystemComponent` _returnvalue (struct :`AttributeName` "MaxRifleReserveAmmo" :`Attribute` "/Script/GASHandsOn.GHOAttributeSetAmmo:MaxRifleReserveAmmo")))))
    (else
      (return false))))

(fn `UserConstructionScript`)